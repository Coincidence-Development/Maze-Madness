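; Player character for a Pac-Man-style arcade game, with continuous four-way movement, an animated mouth and a timed speed boost.
; Axis input latches one direction, which Tick keeps applying once movement is allowed while toggling open and closed meshes.
; The boost swaps speed, material and effects, then reverts after a delay.
; Enemy KilledPlayer dispatchers trigger death, which clears the boost, halts input and plays sound, spin and particles before hiding the player.
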(event `self.ReceiveTick`
  (params (DeltaSeconds :type "Float (single-precision)"))
  (if (`self.bAllowedToMove?`)
    (`|ExecutionSequence`
      (:`then_0`
        ;[0 1 0.1123] Player Gobble Anamation
        (if (`self.bShouldPlayerGobble?`)
          (`KismetSystemLibrary.Delay` 0.05)
          (`/Engine/EditorBlueprintResources/StandardMacros.FlipFlop`
            (:`A`
              _)
            (:`B`
              _))
          (`SceneComponent.ToggleVisibility` (`self.Player_Open`) false)
          (`SceneComponent.ToggleVisibility` (`self.Player_Closed`) false)))
      (:`then_1`
        (if (`self.bGoingUp?`)
          ;[0 1 0.1123] Player Move Up/Down
          (`self.AddMovementInput` (`KismetMathLibrary.GetRightVector` (`KismetMathLibrary.MakeRotator` 0.0 0.0 (.yaw (`self.GetControlRotation`)))) (stale `InputAxis|MoveRight` _output_get) :!label _label)
          (elif (`self.bGoingDown?`)
            (`self.AddMovementInput` (`KismetMathLibrary.GetRightVector` (`KismetMathLibrary.MakeRotator` 0.0 0.0 (.yaw (`self.GetControlRotation`)))) (stale `InputAxis|MoveRight` _output_get_2) :!label _label_2)
            (elif (`self.bGoingLeft?`)
              ;[0 1 0.1123] Player Move Right/Left
              (`self.AddMovementInput` (`KismetMathLibrary.GetForwardVector` (`KismetMathLibrary.MakeRotator` 0.0 0.0 (.yaw (`self.GetControlRotation`)))) (stale `InputAxis|MoveForward` _output_get_2) :!label _label_3)
              (elif (`self.bGoingRight?`)
                (`self.AddMovementInput` (`KismetMathLibrary.GetForwardVector` (`KismetMathLibrary.MakeRotator` 0.0 0.0 (.yaw (`self.GetControlRotation`)))) (stale `InputAxis|MoveForward` _output_get) :!label _label_4)))))))))

(event `InputAxis|MoveRight`
  (params (AxisValue :type "Float (single-precision)"))
  ;[0 1 0.1123] Player Move Up/Down
  (if (>= AxisValue 0.7)
    (set `self.bGoingLeft?` false)
    (set `self.bGoingDown?` false)
    (set `self.bGoingRight?` false)
    (set `self.bGoingUp?` true)
    (bind _output_get (set `self.InputRight` 1.0))
    (goto _label)
    (elif (<= AxisValue -0.7)
      (set `self.bGoingUp?` false)
      (set `self.bGoingRight?` false)
      (set `self.bGoingLeft?` false)
      (set `self.bGoingDown?` true)
      (bind _output_get_2 (set `self.InputRight` -1.0))
      (goto _label_2))))

(event `InputAxis|MoveForward`
  (params (AxisValue :type "Float (single-precision)"))
  ;[0 1 0.1123] Player Move Right/Left
  (if (>= AxisValue 0.7)
    (set `self.bGoingLeft?` false)
    (set `self.bGoingUp?` false)
    (set `self.bGoingDown?` false)
    (set `self.bGoingRight?` true)
    (bind _output_get (set `self.InputForward` 1.0))
    (goto _label_4)
    (elif (<= AxisValue -0.7)
      (set `self.bGoingUp?` false)
      (set `self.bGoingDown?` false)
      (set `self.bGoingRight?` false)
      (set `self.bGoingLeft?` true)
      (bind _output_get_2 (set `self.InputForward` -1.0))
      (goto _label_3))))

(event `UNDO SPEED BOOST`
  ;[0 1 0.1123] Player Was Killed
  ;[0 1 0.1123] Speed Boost
  (set `self.bIsBoosted?` false :!label _label_5)
  (set `CharacterMovementComponent.MaxWalkSpeed` (`self.PlayerRegularSpeed`) (`self.CharacterMovement`))
  (`PrimitiveComponent.SetMaterial` (`self.Player_Open`) 0 "/Game/ArcadeClassic/Materials/M_Base_Inst_Player.M_Base_Inst_Player")
  (`PrimitiveComponent.SetMaterial` (`self.Player_Closed`) 0 "/Game/ArcadeClassic/Materials/M_Base_Inst_Player.M_Base_Inst_Player")
  (`ActorComponent.Deactivate` (`self.VFX_PowerUpSpeed`))
  (`ActorComponent.Deactivate` (`self.SFX_PowerUpSpeed`)))

(event `SPEED BOOST`
  ;[0 1 0.1123] Speed Boost
  (set `self.bIsBoosted?` true)
  (set `CharacterMovementComponent.MaxWalkSpeed` (`self.PlayerBoostedSpeed`) (`self.CharacterMovement`))
  (`PrimitiveComponent.SetMaterial` (`self.Player_Open`) 0 "/Game/ArcadeClassic/Materials/M_Base_Inst_Fruit_Cherries.M_Base_Inst_Fruit_Cherries")
  (`PrimitiveComponent.SetMaterial` (`self.Player_Closed`) 0 "/Game/ArcadeClassic/Materials/M_Base_Inst_Fruit_Cherries.M_Base_Inst_Fruit_Cherries")
  (`ActorComponent.Activate` (`self.VFX_PowerUpSpeed`) false)
  (`ActorComponent.Activate` (`self.SFX_PowerUpSpeed`) false)
  (`KismetSystemLibrary.Delay` 6.0)
  (goto _label_5))

(event `self.ReceiveBeginPlay`
  (`|ExecutionSequence`
    (:`then_1`
      ;[0 1 0.1123] Referance to Enemy Parent
      (bind _outactors (`GameplayStatics.GetAllActorsOfClass` "/Game/ArcadeClassic/Blueprints/Characters/BP_Enemy_Parent.BP_Enemy_Parent_C"))
      (set `self.EnemyParent` _outactors)
      ;[0 1 0.1123] Initalizes Listening of player kill event
      (`self.Listen for player kill`))))

(event `Listen for player kill`
  ;[0 1 0.1123] Lession out for "KilledPlayer" Event Dispatcher
  (add `/Game/ArcadeClassic/Blueprints/Characters/BP_Enemy_Parent.KilledPlayer` (`self.EnemyParent`) (delegate `KilledPlayer_Event_0`)))

(event `KilledPlayer_Event_0`
  ;[0 1 0.1123] Lession out for "KilledPlayer" Event Dispatcher
  (`|ExecutionSequence`
    (:`then_0`
      ;[0 1 0.1123] Kill speed boost effects if boosted
      (`self.UNDO SPEED BOOST`) ; If Player has speed boost effect active when he dies, this will kill it
    )
    (:`then_1`
      ;[0 1 0.1123] Stop Input, navagation, and gobbling
      (`self.DisableInput` (`GameplayStatics.GetPlayerController` 0) null)
      (set `self.bShouldPlayerGobble?` false)
      (set `self.bGoingRight?` false)
      (set `self.bGoingLeft?` false)
      (set `self.bGoingUp?` false)
      (set `self.bGoingDown?` false)
      (set `self.InputRight` 0.0)
      (set `self.InputForward` 0.0)
      (set `CharacterMovementComponent.MaxWalkSpeed` 0.0 (`self.CharacterMovement`)) ; Ensures player has stopped navagation
    )
    (:`then_2`
      ;[0 1 0.1123] Player Death FX
      (`GameplayStatics.PlaySound2D` "/Game/ArcadeClassic/Audio/SFX-Death_Cue.SFX-Death_Cue")
      (`KismetSystemLibrary.Delay` 1.75)
      (`GameplayStatics.SpawnEmitterAtLocation` "/Game/ArcadeClassic/Particles/P_Death.P_Death" (`self.K2_GetActorLocation`) (struct) (3.0 3.0 3.0)) ; Scale X3
      (`self.SetActorHiddenInGame` true))
    (:`then_3`
      ;[0 1 0.1123] Player Death Anamation
      (bind (_direction _player_rotation) (`Timeline|Death Spin` :!via `PlayFromStart`)
        (:`Update`
          (`SceneComponent.K2_SetRelativeRotation` (`self.CapsuleComponent`) (`KismetMathLibrary.MakeRotator` 0.0 0.0 _player_rotation) false false))))))

(fn `UserConstructionScript`)