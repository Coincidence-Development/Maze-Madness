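; Gameplay game mode for a pellet-eating arcade level that manages level completion, bonus spawning and music.
; BeginPlay caches player and enemies, tallies both pellet types, blends to a spawned camera before enabling movement, and spawns one random fruit or speed power-up after a random delay.
; AtePellet counts down to zero, then halts the player and calls LevelCompleted.
; Enemy kill and vulnerability dispatchers switch the music, and level completion stops it.
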(event `AtePellet`
  (bind _player_ref (`self.Player Ref`))
  ;[0 1 0.1123] Level Compleation Check. Runs Script When pellet is eatin
  (bind _result (`/Engine/EditorBlueprintResources/StandardMacros.DecrementInt` (`self.TotalPellets`)) ; Subtract One Pellet
    (:`  `
      (bind _output_get (set `self.TotalPellets` _result)) ; Updated Pellet Ammount
      (if (<= _output_get 0)
        (set `self.bGoodieSpawnOk?` false)
        (`|ExecutionSequence`
          (:`then_0`
            ;[0 1 0.1123] Stop Player Nav
            (`self.DisableInput` (`GameplayStatics.GetPlayerCharacter` 0) (`GameplayStatics.GetPlayerController` 0))
            (set `CharacterMovementComponent.MaxWalkSpeed` 0.0 (`Character.CharacterMovement` _player_ref))
            (set `/Game/ArcadeClassic/Blueprints/Characters/BP_Player.bShouldPlayerGobble?` false _player_ref))
          (:`then_1`
            (`KismetSystemLibrary.PrintString` "END OF LEVEL" true true (struct :`R` 1.0 :`B` 0.551528 :`A` 1.0)))
          (:`then_2`
            (`self.Level Completed`)))))))

(event `self.ReceiveBeginPlay`
  (bind _returnvalue (`GameplayStatics.GetPlayerCharacter` 0))
  (bind _array (`|MakeArray` (`self.GoodieSpawn_01`) (`self.GoodieSpawn_02`)))
  (`|ExecutionSequence`
    (:`then_0`
      ;[0 1 0.1123] Referance to player
      (bind _asbp_player (cast `/Game/ArcadeClassic/Blueprints/Characters/BP_Player` (`GameplayStatics.GetPlayerCharacter` 0)))
      (set `self.Player Ref` _asbp_player)
      ;[0 1 0.1123] Referance to all enemies
      (bind _outactors (`GameplayStatics.GetAllActorsOfClass` "/Game/ArcadeClassic/Blueprints/Characters/BP_Enemy_Parent.BP_Enemy_Parent_C"))
      (set `self.Enemies` _outactors))
    (:`then_2`
      ;[0 1 0.1123] Tally Total Number of Pellets in Level
      (bind _outactors_2 (`GameplayStatics.GetAllActorsOfClass` "/Game/ArcadeClassic/Blueprints/Pickups/BP_Pellet.BP_Pellet_C"))
      (bind _output_get (set `self.TotalRegularPellets` (`KismetArrayLibrary.Array_Length` _outactors_2)))
      (set `self.TotalPellets` (+ _output_get (stale _output_get_2)) :!label _label))
    (:`then_3`
      (bind _outactors_3 (`GameplayStatics.GetAllActorsOfClass` "/Game/ArcadeClassic/Blueprints/Pickups/BP_PowerPellet.BP_PowerPellet_C"))
      (bind _output_get_2 (set `self.TotalPowerPellets` (`KismetArrayLibrary.Array_Length` _outactors_3)))
      (goto _label))
    (:`then_4`
      ;[1 0.9289 0] Gameplay Camera
      (`self.DisableInput` (`GameplayStatics.GetPlayerCharacter` 0) (`GameplayStatics.GetPlayerController` 0))
      (bind _returnvalue_2 (`|SpawnActorFromClass` "/Script/Engine.CameraActor" (`KismetMathLibrary.MakeTransform` (`self.CamGameplay_Loc`) (`self.CamGameplay_Rot`)) "Undefined" "OverrideRootScale" null null))
      (`PlayerController.SetViewTargetWithBlend` (`GameplayStatics.GetPlayerController` 0) _returnvalue_2 6.8 "VTBlend_Linear" 0.0 false)
      (`KismetSystemLibrary.Delay` 7.0)
      (`self.EnableInput` _returnvalue (`GameplayStatics.GetPlayerController` 0))
      (bind _asbp_player_2 (cast `/Game/ArcadeClassic/Blueprints/Characters/BP_Player` _returnvalue))
      (set `/Game/ArcadeClassic/Blueprints/Characters/BP_Player.bAllowedToMove?` true _asbp_player_2))
    (:`then_5`
      ;[0 1 0.1123] Fruit/PowerUp Spawn
      (`KismetSystemLibrary.Delay` (`KismetMathLibrary.RandomFloatInRange` 25.0 50.0))
      (if (`self.bGoodieSpawnOk?`)
        (bind _output_get_3 (set `self.GoodieSpawnLocation` _array))
        (switch `int` (`KismetMathLibrary.RandomIntegerInRange` 0 2)
          (:`0`
            (bind _returnvalue_3 (`KismetMathLibrary.Conv_VectorToTransform` (`|GetArrayItem` _output_get_3 (`KismetMathLibrary.RandomIntegerInRange` 0 (- (`KismetArrayLibrary.Array_Length` _array) 1)))))
            (`|SpawnActorFromClass` "/Game/ArcadeClassic/Blueprints/Pickups/BP_Food_Cherry.BP_Food_Cherry_C" _returnvalue_3 "Undefined" "OverrideRootScale" null null))
          (:`1`
            (`|SpawnActorFromClass` "/Game/ArcadeClassic/Blueprints/Pickups/BP_Food_Orange.BP_Food_Orange_C" _returnvalue_3 "Undefined" "OverrideRootScale" null null))
          (:`2`
            (`|SpawnActorFromClass` "/Game/ArcadeClassic/Blueprints/Pickups/BP_PowerUp_Speed.BP_PowerUp_Speed_C" _returnvalue_3 "Undefined" "OverrideRootScale" null null)))))
    (:`then_6`
      (`|ExecutionSequence`
        (:`then_0`
          ;[0 1 0.1123] Music Stops / Resumes when player is killed
          (add `/Game/ArcadeClassic/Blueprints/Characters/BP_Enemy_Parent.KilledPlayer` (`self.Enemies`) (delegate `KilledPlayer_Event_0`)))
        (:`then_1`
          ;[0 1 0.1123] Enimies Vulnerable or not
          (add `/Game/ArcadeClassic/Blueprints/Characters/BP_Enemy_Parent.Vulnerable` (`self.Enemies`) (delegate `Vulnerable_Event_0`)))
        (:`then_2`
          (add `/Game/ArcadeClassic/Blueprints/Characters/BP_Enemy_Parent.Not Vulnerable` (`self.Enemies`) (delegate `Not Vulnerable_Event_0`)))
        (:`then_3`
          ;[0 1 0.1123] Level Complete (Stop Music)
          (add `self.Level Completed` (delegate `Level Completed_Event`)))))))

(event `KilledPlayer_Event_0`
  (bind _music_gameplay (`self.Music_Gameplay`))
  ;[0 1 0.1123] Music Stops / Resumes when player is killed
  (`|ExecutionSequence`
    (:`then_0`
      (`AudioComponent.Stop` _music_gameplay))
    (:`then_1`
      (`KismetSystemLibrary.Delay` 7.0)
      (`AudioComponent.FadeIn` _music_gameplay 0.5 1.0 7.0))))

(event `Vulnerable_Event_0`
  (bind _music_vulnerable (`self.Music_Vulnerable`))
  ;[0 1 0.1123] Enimies Vulnerable or not
  (`AudioComponent.SetPaused` (`self.Music_Gameplay`) true)
  (if (not (`AudioComponent.IsPlaying` _music_vulnerable))
    (`AudioComponent.Play` _music_vulnerable 0.0)))

(event `Not Vulnerable_Event_0`
  ;[0 1 0.1123] Enimies Vulnerable or not
  (`AudioComponent.SetPaused` (`self.Music_Gameplay`) false) ; Unpause Gameplay Music
  (`AudioComponent.Stop` (`self.Music_Vulnerable`)) ; Stop Vulnerable Music
)

(event `Level Completed_Event`
  ;[0 1 0.1123] Level Complete (Stop Music)
  (`KismetSystemLibrary.Delay` 0.1)
  (`AudioComponent.Stop` (`self.Music_Gameplay`))
  (`AudioComponent.Stop` (`self.Music_Vulnerable`)))

(fn `UserConstructionScript`)